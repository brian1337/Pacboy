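; Main player character Blueprint that creates the test HUD, toggles the mouse cursor on Escape and shows an overhead name and health bar.
; BeginPlay registers the character in GM_TestGameMode's Characters list and applies the blue hero mesh on authority.
; Tick updates the bar from PlayerState and Health, then yaws other listed characters' bars toward this one.
; On death, it destroys the bar and leaves the list once.
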(event `Key|Escape`
  (bind _returnvalue (`self.GetController`))
  (:`Pressed`
    (if (`self.EscapeOn`)
      (set `self.EscapeOn` false)
      (bind _returnvalue_2 (`Controller.CastToPlayerController` _returnvalue))
      (set `PlayerController.bShowMouseCursor` false _returnvalue_2)
      (else
        (set `self.EscapeOn` true)
        (bind _returnvalue_3 (`Controller.CastToPlayerController` _returnvalue))
        (set `PlayerController.bShowMouseCursor` true _returnvalue_3)))))

(event `self.ReceiveBeginPlay`
  (bind _returnvalue (`|CreateWidget` "/Game/HUD/TestGameWidgets.TestGameWidgets_C"))
  (`UserWidget.AddToViewport` _returnvalue)
  (`KismetSystemLibrary.Delay` 0.1)
  (bind _asgm_test_game_mode (cast `/Game/GameModes/GM_TestGameMode` (`GameplayStatics.GetGameMode`)))
  (bind _characters (`/Game/GameModes/GM_TestGameMode.Characters` _asgm_test_game_mode))
  (if (not (`KismetArrayLibrary.Array_Contains` _characters self))
    (`KismetArrayLibrary.Array_Add` _characters self))
  (`/Engine/EditorBlueprintResources/ActorMacros.Switch Has Authority`
    (:`Authority`
      (`self.RecolorSelf`))))

(event `RecolorSelf`
  (`SkinnedMeshComponent.SetSkinnedAssetAndUpdate` "/Game/Characters/HeroTPP/HeroTPP_Blue.HeroTPP_Blue"))

(event `self.ReceiveTick`
  (params (DeltaSeconds :type "Float (single-precision)"))
  (bind _playername (`PlayerState.PlayerName` (`self.PlayerState`)))
  (if (`self.bIsDead`)
    (`/Engine/EditorBlueprintResources/StandardMacros.DoOnce` false
      (:`Completed`
        (`ActorComponent.K2_DestroyComponent` (`self.BarScene`))
        (bind _asgm_test_game_mode (cast `/Game/GameModes/GM_TestGameMode` (`GameplayStatics.GetGameMode`)))
        (`KismetArrayLibrary.Array_RemoveItem` (`/Game/GameModes/GM_TestGameMode.Characters` _asgm_test_game_mode) self)))
    (else
      (bind _aswidget_player_info (cast `/Game/HUD/WIDGET_PlayerInfo` (`WidgetComponent.GetUserWidgetObject` (`self.HP_Widget`))))
      (bind _playername_2 (`/Game/HUD/WIDGET_PlayerInfo.PlayerName` _aswidget_player_info))
      (if (not (`KismetStringLibrary.EqualEqual_StrStr` _playername (`KismetStringLibrary.Conv_ObjectToString` _playername_2)))
        (`TextBlock.SetText` _playername_2 (`KismetTextLibrary.Conv_StringToText` _playername)))
      (`ProgressBar.SetPercent` (`/Game/HUD/WIDGET_PlayerInfo.HealthBar` _aswidget_player_info) (/ (`self.Health`) 100.0))
      (bind _asgm_test_game_mode_2 (cast `/Game/GameModes/GM_TestGameMode` (`GameplayStatics.GetGameMode`)))
      (for _array_element (`/Game/GameModes/GM_TestGameMode.Characters` _asgm_test_game_mode_2)
        (if (!= _array_element self)
          (`self.RotateHealthBar` _array_element))))))

(event `RotateHealthBar`
  (params (Character :type "/Game/Characters/BP_MainCharacter Object Reference"))
  (bind _barscene (`/Game/Characters/BP_MainCharacter.BarScene` Character))
  (`SceneComponent.K2_SetWorldRotation` _barscene (`KismetMathLibrary.MakeRot` 0.0 (.yaw (`KismetMathLibrary.FindLookAtRotation` (`SceneComponent.K2_GetComponentLocation` _barscene) (`self.K2_GetActorLocation` self)))) false))

(fn `UserConstructionScript`)