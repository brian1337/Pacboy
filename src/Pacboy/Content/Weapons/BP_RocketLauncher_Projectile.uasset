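; Rocket launcher projectile that handles the explosion when the rocket hits.
; OnImpact spawns the impact particle effect with its pitch turned 180 degrees from the projectile's rotation and plays an explosion sound at that location.
; It then applies radial damage credited to the Shooter controller, using WorldStatic as the damage prevention channel so that blocking geometry shields targets.
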(event `self.OnImpact`
  (params (OtherActor :type "Actor Object Reference") (OtherComp :type "PrimitiveComponent Object Reference"))
  (bind _returnvalue (`self.K2_GetActorLocation`))
  (`GameplayStatics.SpawnEmitterAtLocation` "/Game/Effects/ParticleSystems/Weapons/RocketLauncher/Impact/P_Launcher_IH.P_Launcher_IH" _returnvalue (`KismetMathLibrary.MakeRot` (+ (.pitch (`self.K2_GetActorRotation`)) 180.0) (.yaw (`self.K2_GetActorRotation`)) (.roll (`self.K2_GetActorRotation`))))
  (`GameplayStatics.PlaySoundAtLocation` "/Game/Sounds/Weapon_GrenadeLauncher/Mono/GrenadeLauncher_Explosion_Cue.GrenadeLauncher_Explosion_Cue" _returnvalue)
  (`GameplayStatics.ApplyRadialDamage` :`BaseDamage` 100.0 :`Origin` (`self.K2_GetActorLocation`) :`DamageRadius` 375.0 :`DamageTypeClass` "/Script/Engine.DamageType" :`DamageCauser` self :`InstigatedByController` (`self.Shooter`) :`DamagePreventionChannel` "ECC_WorldStatic"))

(fn `UserConstructionScript`)